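; Actor that plays a branching dialogue cinematic at its transform, using main and response Level Sequence players.
; Starts the entry sequence, with play and pause events bound for transform offsetting and branching.
; ProceedAfterSequence filters transitions through Chronicle rules, then stops, auto-continues, or loops the response sequence while Tick polls three choice keys.
; Choices raise Chronicle callbacks and synchronously load the next sequence, starting at its node's frame.
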(event `self.ReceiveBeginPlay`
  (`self.CachePlayers`)
  (`self.InitializePlayers`)
  (`self.StartCinematic`))

(event `self.ReceiveTick`
  (params (DeltaSeconds :type "Float (single-precision)"))
  (`self.TryReadingResponse`))

(fn `CachePlayers`
  (bind _aslevel_sequence_actor (cast `LevelSequenceActor` (`ChildActorComponent.ChildActor` (`self.MainLevelSequenceActor`))))
  (set `self.MainPlayer` _aslevel_sequence_actor)
  (bind _aslevel_sequence_actor_2 (cast `LevelSequenceActor` (`ChildActorComponent.ChildActor` (`self.ResponseLevelSequenceActor`))))
  (set `self.ResponsePlayer` _aslevel_sequence_actor_2))

(fn `InitializePlayers`
  (bind _sequenceplayer (`LevelSequenceActor.SequencePlayer` (`self.MainPlayer`)))
  (add `MovieSceneSequencePlayer.OnPause` _sequenceplayer (`|CreateDelegate` :!event `ProceedAfterSequence`))
  (add `MovieSceneSequencePlayer.OnPlay` _sequenceplayer (`|CreateDelegate` :!event `InitMainPlayer`))
  (add `MovieSceneSequencePlayer.OnPlay` (`LevelSequenceActor.SequencePlayer` (`self.ResponsePlayer`)) (`|CreateDelegate` :!event `InitResponsePlayer`)))

(fn `InitMainPlayer`
  (`Chronicle_PlaybackFunctionLibrary.OffsetSpawnableTransforms` (`self.MainPlayer`) (.location (`self.GetTransform`)) (.rotation (`self.GetTransform`))))

(fn `InitResponsePlayer`
  (`Chronicle_PlaybackFunctionLibrary.OffsetResponseCamera` (`self.ResponsePlayer`) (`self.ResponseCameraTransform`) (.location (`self.GetTransform`)) (.rotation (`self.GetTransform`))))

(fn `ProceedAfterSequence`
  (bind _availabletransitions (`self.AvailableTransitions`))
  (`KismetArrayLibrary.Array_Clear` (`self.AvailableTransitions`))
  (for _array_element (`.Transitions` (break `Chronicle_SequenceInfo` (`BlueprintMapLibrary.Map_Find` (`.SequencesById` (break `Chronicle_DialogueInfo` (`self.Info`))) (`self.SequenceId`))))
    (bind _returnvalue (`Chronicle_RuleSubsystem.Resolve` (subsystem `Chronicle_RuleSubsystem`) (`.Rules` (break `Chronicle_TransitionInfo` _array_element))))
    (if _returnvalue
      (`KismetArrayLibrary.Array_Add` (`self.AvailableTransitions`) _array_element)))
  (for (_array_element_2 _array_index) _availabletransitions
    (switch `EChronicle_TransitionType` (`.Type` (break `Chronicle_TransitionInfo` _array_element_2))
      (:`Game`
        (`MovieSceneSequencePlayer.Stop` (`LevelSequenceActor.SequencePlayer` (`self.MainPlayer`))))
      (:`Response`
        (if (not (`|EnumEquality` (`.Type` (break `Chronicle_TransitionInfo` (`|GetArrayItem` (`self.AvailableTransitions`)))) "AutoContinue"))
          (`self.StartReadingResponse`)))
      (:`AutoContinue`
        (`self.ReadResponse` _array_index))))
  (if (`KismetArrayLibrary.Array_IsEmpty` _availabletransitions)
    (`MovieSceneSequencePlayer.Stop` (`LevelSequenceActor.SequencePlayer` (`self.MainPlayer`)))))

(fn `ReadResponse`
  (params (TransitionIndex :type Integer))
  (bind _output (`|GetArrayItem` (`self.AvailableTransitions`) TransitionIndex))
  (bind ((`Callbacks` _callbacks) (`SequenceId` _sequenceid)) (break `Chronicle_TransitionInfo` _output))
  (bind ((`SequenceId` _sequenceid_2) (`NodeId` _nodeid)) (break `Chronicle_TransitionInfo` _output))
  (bind _value (`BlueprintMapLibrary.Map_Find` (`.SequencesById` (break `Chronicle_DialogueInfo` (`self.Info`))) _sequenceid_2))
  (bind ((`Sequence` _sequence)) (break `Chronicle_SequenceInfo` _value))
  (`KismetSystemLibrary.LoadAsset_Blocking` _sequence)
  (`Chronicle_RuleSubsystem.Raise` (subsystem `Chronicle_RuleSubsystem`) _callbacks)
  (`LevelSequenceActor.SetSequence` (`self.MainPlayer`) (`|ConvertAsset` _sequence))
  (`Chronicle_PlaybackFunctionLibrary.SetPlaybackPosition` (`self.MainPlayer`) (`BlueprintMapLibrary.Map_Find` (`.StartFrameByNodeIds` (break `Chronicle_SequenceInfo` _value)) _nodeid))
  (`MovieSceneSequencePlayer.Play` (`LevelSequenceActor.SequencePlayer` (`self.MainPlayer`)))
  (set `self.SequenceId` _sequenceid))

(fn `StartCinematic`
  (bind ((`SequencesById` _sequencesbyid) (`EntrySequenceId` _entrysequenceid)) (break `Chronicle_DialogueInfo` (`self.Info`)))
  (bind ((`Sequence` _sequence)) (break `Chronicle_SequenceInfo` (`BlueprintMapLibrary.Map_Find` _sequencesbyid _entrysequenceid)))
  (`KismetSystemLibrary.LoadAsset_Blocking` _sequence)
  (`LevelSequenceActor.SetSequence` (`self.MainPlayer`) (`|ConvertAsset` _sequence))
  (`MovieSceneSequencePlayer.Play` (`LevelSequenceActor.SequencePlayer` (`self.MainPlayer`)))
  (set `self.SequenceId` (`.EntrySequenceId` (break `Chronicle_DialogueInfo` (`self.Info`)))))

(fn `StartReadingResponse`
  (set `self.IsAcceptingResponses` true)
  (`MovieSceneSequencePlayer.PlayLooping` (`LevelSequenceActor.SequencePlayer` (`self.ResponsePlayer`)) -1))

(fn `TryReadingResponse`
  (bind _returnvalue (`GameplayStatics.GetPlayerController` 0))
  (if (`self.IsAcceptingResponses`)
    (if (`PlayerController.IsInputKeyDown` _returnvalue "One")
      (`self.ReadResponse` 0)
      (set `self.IsAcceptingResponses` false :!label _label)
      (`MovieSceneSequencePlayer.Stop` (`LevelSequenceActor.SequencePlayer` (`self.ResponsePlayer`)))
      (elif (`PlayerController.IsInputKeyDown` _returnvalue "Two")
        (`self.ReadResponse` 1)
        (goto _label)
        (elif (`PlayerController.IsInputKeyDown` _returnvalue "Three")
          (`self.ReadResponse` 2)
          (goto _label))))))

(fn `UserConstructionScript`
  (for _array_element (`self.CameraTransforms`)
    _))